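; Project template helper functions for setting the DLSS mode and interpolating Vector2D values.
; SetDLSSMode toggles DLSS, queries mode information at the primary monitor's resolution, and issues r.ScreenPercentage console commands for optimal and min/max values, zeroing the bounds for fixed-percentage modes.
; LerpVector2D, despite its name, blends each input's own components: X from A.X to A.Y, Y from B.X to B.Y.
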(fn `Lerp (Vector2D)`
  (params (A :type "Vector2D Structure") (B :type "Vector2D Structure") (Alpha :type "Float (double-precision)"))
  (returns (`Return Value` :type "Vector2D Structure"))
  (bind (_x _y) (`KismetMathLibrary.BreakVector2D` B))
  (bind (_x_2 _y_2) (`KismetMathLibrary.BreakVector2D` A))
  (return (`KismetMathLibrary.MakeVector2D` (`KismetMathLibrary.Lerp` _x_2 _y_2 Alpha) (`KismetMathLibrary.Lerp` _x _y Alpha))))

(fn `Set DLSS Mode`
  (params (`Mode to set` :type "UDLSSMode Enum" :default "Off"))
  (bind (_width _height) (`LowEntryExtendedStandardLibrary.GetPrimaryMonitorResolution`))
  (bind (_bissupported _optimalscreenpercentage _bisfixedscreenpercentage _minscreenpercentage _maxscreenpercentage) (`DLSSLibrary.GetDLSSModeInformation` `Mode to set` (`KismetMathLibrary.MakeVector2D` (`KismetMathLibrary.Conv_IntToDouble` _width) (`KismetMathLibrary.Conv_IntToDouble` _height))))
  (`DLSSLibrary.EnableDLSS` (select `UDLSSMode` `Mode to set` :`Auto` true :`UltraQuality` true :`Quality` true :`Balanced` true :`Performance` true :`UltraPerformance` true))
  (if _bisfixedscreenpercentage
    (`KismetSystemLibrary.ExecuteConsoleCommand` null (`KismetStringLibrary.Concat_StrStr` "r.ScreenPercentage.MaxResolution" "0") null)
    (`KismetSystemLibrary.ExecuteConsoleCommand` null (`KismetStringLibrary.Concat_StrStr` "r.ScreenPercentage.MinResolution" "0") null)
    (else
      (`KismetSystemLibrary.ExecuteConsoleCommand` null (`KismetStringLibrary.Concat_StrStr` "r.ScreenPercentage.MaxResolution" (`KismetStringLibrary.Conv_IntToString` (`KismetMathLibrary.FTrunc` (* (`.Height` (`LowEntryExtendedStandardLibrary.GetPrimaryMonitorResolution`)) _maxscreenpercentage)))) null)
      (`KismetSystemLibrary.ExecuteConsoleCommand` null (`KismetStringLibrary.Concat_StrStr` "r.ScreenPercentage.MinResolution" (`KismetStringLibrary.Conv_IntToString` (`KismetMathLibrary.FTrunc` (* (`.Height` (`LowEntryExtendedStandardLibrary.GetPrimaryMonitorResolution`)) _minscreenpercentage)))) null)))
  (`KismetSystemLibrary.ExecuteConsoleCommand` null (`KismetStringLibrary.Concat_StrStr` "r.ScreenPercentage" (`KismetStringLibrary.Conv_DoubleToString` _optimalscreenpercentage)) null)
  (return))