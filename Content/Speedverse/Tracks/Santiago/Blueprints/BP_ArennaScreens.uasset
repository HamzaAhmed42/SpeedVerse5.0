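; Arena screen actor for the Santiago track that switches its RectLight on at night and off by day.
; On BeginPlay it takes the first Ultra Dynamic Sky actor in the level and binds to its sunset and sunrise events.
; Sunset shows the light and propagates to child components, while sunrise hides only the RectLight itself.
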(event `self.ReceiveBeginPlay`
  (bind _outactors (`GameplayStatics.GetAllActorsOfClass` "/Game/UltraDynamicSky/Blueprints/Ultra_Dynamic_Sky.Ultra_Dynamic_Sky_C"))
  (bind _output_get (set `self.UDS` (`|GetArrayItem` _outactors)))
  (add `/Game/UltraDynamicSky/Blueprints/Ultra_Dynamic_Sky.Sunset` _output_get (delegate `Turn On Street Lights_Event`))
  (add `/Game/UltraDynamicSky/Blueprints/Ultra_Dynamic_Sky.Sunrise` (`self.UDS`) (delegate `Turn Off Street Lights_Event`)))

(event `Turn On Street Lights_Event`
  (`SceneComponent.SetVisibility` (`self.RectLight`) true true))

(event `Turn Off Street Lights_Event`
  (`SceneComponent.SetVisibility` (`self.RectLight`) false false))

(fn `UserConstructionScript`)