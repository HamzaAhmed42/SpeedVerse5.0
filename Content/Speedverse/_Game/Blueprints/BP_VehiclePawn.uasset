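; BP_VehiclePawn is a vehicle pawn that leaves tyre marks while braking.
; Each tick with BreakPressed set, it spawns scaled-down BP_TyreMarks actors at the TyreMarksR and TyreMarksL components, aligned to the pawn's rotation.
; A short Delay on the same Tick path then destroys one BP_TyreMarks found by class, so removal runs slower than spawning and is not tied to the pair just spawned.
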(event `self.ReceiveTick`
  (params (DeltaSeconds :type "Float (single-precision)"))
  (if (`self.bBreakPressed`)
    (`|SpawnActorFromClass` "/Game/Speedverse/_Game/Blueprints/BP_TyreMarks.BP_TyreMarks_C" (`KismetMathLibrary.MakeTransform` (`SceneComponent.K2_GetComponentLocation` (`self.TyreMarks_R`)) (`self.K2_GetActorRotation`) (0.2 0.2 0.2)) "Undefined" "OverrideRootScale" null null)
    (`|SpawnActorFromClass` "/Game/Speedverse/_Game/Blueprints/BP_TyreMarks.BP_TyreMarks_C" (`KismetMathLibrary.MakeTransform` (`SceneComponent.K2_GetComponentLocation` (`self.TyreMarks_L`)) (`self.K2_GetActorRotation`) (0.2 0.2 0.2)) "Undefined" "OverrideRootScale" null null)
    (`KismetSystemLibrary.Delay` 0.2)
    (bind _returnvalue (`GameplayStatics.GetActorOfClass` "/Game/Speedverse/_Game/Blueprints/BP_TyreMarks.BP_TyreMarks_C"))
    (`self.K2_DestroyActor` _returnvalue)))

(fn `UserConstructionScript`)