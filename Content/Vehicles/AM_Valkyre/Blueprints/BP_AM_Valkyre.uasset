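; Player-driven Valkyre car Blueprint on Chaos wheeled vehicle movement, with engine toggle, throttle, brake, steering and handbrake input.
; Throttle and brake respond only while the engine runs; angular damping rises when airborne.
; Tick eases third-person zoom, prints driving-state debug and drives RPM-based engine audio, while gear changes trigger gearbox and exhaust sounds.
; A switchable first-person camera adds clamped free look, and the chase camera can auto-rotate with movement.
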(event `self.ReceiveBeginPlay`
  ;[0 0.8166 1 1 50] Initialization Vehicle And Camera Zoom
  (`|ExecutionSequence`
    (:`then_0`
      (`KismetSystemLibrary.ExecuteConsoleCommand` "r.motionblur.amount 0" null))
    (:`then_1`
      (`self.Init_Vehicle_Movement_Component`)
      (`self.Init_Camera_Zoom`))))

(event `self.ReceiveTick`
  (params (DeltaSeconds :type "Float (single-precision)"))
  ;[1 0.5451 0] Update Wheels And Camera Zoom
  (`self.Set_Angular_Damping`)
  (`self.Update_Camera_Zoom`)
  (`|ExecutionSequence`
    (:`then_0`
      ;[0 0 0] ALL DEBUG
      (bind (_throttle _brakes _steering _forward_speed_km_h _rpm _current_gear _automatic_transmission _all_wheels_on_surface _no_wheels_on_surface _handbrake) (`self.Get_All_Driving_State_Vehicle`))
      (`self.All_Debug` _throttle _brakes _steering _forward_speed_km_h _rpm _current_gear 0.0 0.0 0.0 0.0 _automatic_transmission _handbrake))
    (:`then_1`
      ;[0 0.1392 1] Update Engine Sounds
      (`self.Set_Engine_Sounds`))))

(event `InputAction|Start Engine Input`
  (params (Key :type "Key Structure"))
  ;[1 0 0 1 50] KEYBOARD INPUTS
  ;;[1 0.197 0.1547] Start Engine Input "T" Button
  (:`Pressed`
    (`self.Set_Start_Engine_Input`)))

(event `InputAxis|Move Forward Input`
  (params (AxisValue :type "Float (single-precision)"))
  ;[1 0 0 1 50] KEYBOARD INPUTS
  ;;[1 0.197 0.1547] Move Forward Input
  (if (`self.bIs_Engine_Start?`)
    (bind _output_get (set `self.Move_Forward` AxisValue))
    (set `self.bIs_Vehicle_Moving_Forward?` (< 0.1 _output_get))
    (`self.Set Move Forward` (`self.Move_Forward`))
    ;[0 0.245 1] Gearbox And Exhaust Sounds
    (`self.Set_Gearbox_Exhaust_Sounds`)))

(event `InputAxis|Steering Input`
  (params (AxisValue :type "Float (single-precision)"))
  ;[1 0 0 1 50] KEYBOARD INPUTS
  ;;[1 0.197 0.1547] Steering Input
  (`self.Set Steering Update Input` AxisValue))

(event `InputAction|Handbrake Input`
  (params (Key :type "Key Structure"))
  (bind _vehiclemovementcomponent (`self.VehicleMovementComponent`))
  ;[1 0 0 1 50] KEYBOARD INPUTS
  ;;[1 0.197 0.1547] Handbrake Input "Space" Button
  (:`Pressed`
    (`ChaosVehicleMovementComponent.SetHandbrakeInput` _vehiclemovementcomponent true))
  (:`Released`
    (`ChaosVehicleMovementComponent.SetHandbrakeInput` _vehiclemovementcomponent false)))

(event `InputAxis|Look Right Input`
  (params (AxisValue :type "Float (single-precision)"))
  ;[1 0 0 1 50] KEYBOARD INPUTS
  ;;[1 0.197 0.1547] Camera Rotation Input
  (`self.Set_Camera_Look_Around` (stale `InputAxis|Look Up Input` AxisValue) AxisValue :!label _label))

(event `InputAxis|Look Up Input`
  (params (AxisValue :type "Float (single-precision)"))
  ;[1 0 0 1 50] KEYBOARD INPUTS
  ;;[1 0.197 0.1547] Camera Rotation Input
  (goto _label))

(event `InputAction|Switch Camera Input`
  (params (Key :type "Key Structure"))
  ;[1 0 0 1 50] KEYBOARD INPUTS
  ;;[1 0.197 0.1547] Switch Camera Input "TAB" Button
  (:`Pressed`
    (`self.Set_Switch_Camera` false)))

(event `Key|MouseScrollDown`
  (params (Key :type "Key Structure"))
  (bind (_camera_zoom_bounds_x _camera_zoom_bounds_y) (`KismetMathLibrary.BreakVector2D` (`self.Camera_Zoom_Bounds`)))
  ;[1 0 0 1 50] KEYBOARD INPUTS
  ;;[1 0.197 0.1547] Smooth Camera Zoom Input
  (:`Pressed`
    (`/Engine/EditorBlueprintResources/StandardMacros.IncrementFloat` (`self.Camera_Zoom_Multiplier`)
      (:`  `
        (set `self.Camera_Zoom_Multiplier` (`KismetMathLibrary.FClamp` (`self.Camera_Zoom_Multiplier`) _camera_zoom_bounds_x _camera_zoom_bounds_y))))))

(event `Key|MouseScrollUp`
  (params (Key :type "Key Structure"))
  (bind (_camera_zoom_bounds_x _camera_zoom_bounds_y) (`KismetMathLibrary.BreakVector2D` (`self.Camera_Zoom_Bounds`)))
  ;[1 0 0 1 50] KEYBOARD INPUTS
  ;;[1 0.197 0.1547] Smooth Camera Zoom Input
  (:`Pressed`
    (`/Engine/EditorBlueprintResources/StandardMacros.DecrementFloat` (`self.Camera_Zoom_Multiplier`)
      (:`  `
        (set `self.Camera_Zoom_Multiplier` (`KismetMathLibrary.FClamp` (`self.Camera_Zoom_Multiplier`) _camera_zoom_bounds_x _camera_zoom_bounds_y))))))

(fn `Get_All_Driving_State_Vehicle`
  (returns (Throttle :type "Float (single-precision)") (Brakes :type "Float (single-precision)") (Steering :type "Float (single-precision)") (`Forward_Speed_KM/H` :type "Float (double-precision)") (RPM :type "Float (single-precision)") (Current_Gear :type Integer) (Automatic_Transmission :type Boolean) (All_Wheels_On_Surface :type Boolean) (No_Wheels_On_Surface :type Boolean) (Handbrake :type Boolean))
  (bind _vehiclemovementcomponent (`self.VehicleMovementComponent`))
  (bind _returnvalue (`ChaosVehicleMovementComponent.GetThrottleInput` _vehiclemovementcomponent))
  (bind _returnvalue_2 (`ChaosVehicleMovementComponent.GetBrakeInput` _vehiclemovementcomponent))
  (bind _returnvalue_3 (`ChaosVehicleMovementComponent.GetSteeringInput` _vehiclemovementcomponent))
  (bind _aschaos_wheeled_vehicle_movement_component (cast `ChaosWheeledVehicleMovementComponent` _vehiclemovementcomponent))
  (bind _value (`self.Get_Status_Wheels_On_Surface` _aschaos_wheeled_vehicle_movement_component))
  (return _returnvalue _returnvalue_2 _returnvalue_3 (* (`KismetMathLibrary.Abs` (`ChaosVehicleMovementComponent.GetForwardSpeed` _vehiclemovementcomponent)) 0.036) (`ChaosWheeledVehicleMovementComponent.GetEngineRotationSpeed` _aschaos_wheeled_vehicle_movement_component) (`ChaosVehicleMovementComponent.GetCurrentGear` _vehiclemovementcomponent) (`ChaosVehicleMovementComponent.GetUseAutoGears` _vehiclemovementcomponent) (== _value (`ChaosWheeledVehicleMovementComponent.GetNumWheels` _aschaos_wheeled_vehicle_movement_component)) (== _value 0) (`ChaosVehicleMovementComponent.GetHandbrakeInput` _vehiclemovementcomponent)))

(fn `Get_Status_Wheels_On_Surface`
  (params (Wheels_State :type "ChaosWheeledVehicleMovementComponent Object Reference"))
  (returns (Value :type Integer))
  (for _index (range (`ChaosWheeledVehicleMovementComponent.GetNumWheels` Wheels_State))
    (if (`ChaosWheeledVehicleMovementComponent.BreakWheelStatus` (`ChaosWheeledVehicleMovementComponent.GetWheelState` Wheels_State _index))
      (set `self.Num_Wheels_On_Surface` (+ (`self.Num_Wheels_On_Surface`) 1))))
  (return (`self.Num_Wheels_On_Surface`)))

(fn `Init_Camera_Zoom`
  ;[1 1 1] Init Camera Zoom
  (set `SpringArmComponent.TargetArmLength` (* (`self.Camera_Zoom_Step`) (`self.Camera_Zoom_Multiplier`)) (`self.TP_SpringArm`)))

(fn `Init_Vehicle_Movement_Component`
  (returns (Get_Ref_Chaos_Wheeled_Vehicle_Movement_Component :type "ChaosWheeledVehicleMovementComponent Object Reference"))
  (bind _aschaos_wheeled_vehicle_movement_component (cast `ChaosWheeledVehicleMovementComponent` (`self.VehicleMovementComponent`)))
  (bind _output_get (set `self.Ref_Chaos_Wheeled_Vehicle_Movement_Component` _aschaos_wheeled_vehicle_movement_component))
  (return _output_get))

(fn `Set Move Forward`
  (params (Move_Forward_Axis_Input :type "Float (single-precision)"))
  (bind _vehiclemovementcomponent (`self.VehicleMovementComponent`))
  (if (>= Move_Forward_Axis_Input 0.0)
    (`ChaosVehicleMovementComponent.SetThrottleInput` _vehiclemovementcomponent Move_Forward_Axis_Input)
    (set `self.bIs_Brakes?` false)
    (`ChaosVehicleMovementComponent.SetBrakeInput` _vehiclemovementcomponent 0.0)
    (set `self.bIs_Brakes?` true)
    (else
      (`ChaosVehicleMovementComponent.SetBrakeInput` _vehiclemovementcomponent (* Move_Forward_Axis_Input -1.0))
      (set `self.bIs_Brakes?` true)
      (`ChaosVehicleMovementComponent.SetThrottleInput` _vehiclemovementcomponent 0.0)
      (set `self.bIs_Brakes?` false)))
  (return))

(fn `Set Steering Update Input`
  (params (Steering :type "Float (single-precision)" :default 0.0))
  (bind _vehiclemovementcomponent (`self.VehicleMovementComponent`))
  ;[0.02042 1 0 1 30] Steering Wheel Interior
  (bind _aschaos_wheeled_vehicle_movement_component (cast `ChaosWheeledVehicleMovementComponent` _vehiclemovementcomponent))
  (bind _wheels (`ChaosWheeledVehicleMovementComponent.Wheels` _aschaos_wheeled_vehicle_movement_component))
  (bind _returnvalue (`ChaosVehicleWheel.GetSteerAngle` (`|GetArrayItem` _wheels)))
  (bind _returnvalue_2 (`ChaosVehicleWheel.GetSteerAngle` (`|GetArrayItem` _wheels 1)))
  (set `self.Interior_Steering_Wheel_Angle` (`KismetMathLibrary.SelectFloat` (* _returnvalue 5.0) (* _returnvalue_2 5.0) (> (`KismetMathLibrary.Abs` _returnvalue) (`KismetMathLibrary.Abs` _returnvalue_2))))
  (`ChaosVehicleMovementComponent.SetSteeringInput` _vehiclemovementcomponent Steering))

(fn `Set_Angular_Damping`
  ;[1 0 0.8109] Movement component setup
  (`PrimitiveComponent.SetAngularDamping` (`self.Mesh`) (`KismetMathLibrary.SelectFloat` 0.0 3.0 (`NavMovementComponent.IsMovingOnGround` (`self.Ref_Chaos_Wheeled_Vehicle_Movement_Component`)))) ; Damps rotation when in air
)

(fn `Set_Camera_Look_Around`
  (params (`Delta Rotation Y (Pitch)` :type "Float (single-precision)") (`Delta Rotation Z (Yaw)` :type "Float (single-precision)"))
  (bind _spring_arm_first_person_camera (`self.Spring_Arm_First_Person_Camera`))
  (bind _tp_springarm (`self.TP_SpringArm`))
  (bind (_relativelocation_x _relativelocation_y _relativelocation_z) (`KismetMathLibrary.BreakVector` (`SceneComponent.RelativeLocation` _spring_arm_first_person_camera)))
  (bind (_relativerotation_roll _relativerotation_pitch _relativerotation_yaw) (`KismetMathLibrary.BreakRotator` (`SceneComponent.RelativeRotation` _spring_arm_first_person_camera)))
  (bind (_relativerotation_roll_2 _relativerotation_pitch_2 _relativerotation_yaw_2) (`KismetMathLibrary.BreakRotator` (`SceneComponent.RelativeRotation` _tp_springarm)))
  ;[0 1 0.06954] Third Person (Back) Camera
  (`SceneComponent.K2_AddRelativeRotation` _tp_springarm (`KismetMathLibrary.MakeRotator` 0.0 (`self.GetInputAxisValue`) (`self.GetInputAxisValue`)) false false)
  (`SceneComponent.K2_SetRelativeRotation` _tp_springarm (`KismetMathLibrary.SelectRotator` (`KismetMathLibrary.SelectRotator` (struct :`Pitch` -15.0 :`Yaw` 180.0) (struct :`Pitch` -15.0) (`self.bIs_Camera_Look_Back?`)) (`KismetMathLibrary.MakeRotator` 0.0 (`KismetMathLibrary.FClamp` _relativerotation_pitch_2 -50.0 30.0) _relativerotation_yaw_2) (and (`self.bIs_Auto_Rotate_Back_Camera?`) (not (`KismetMathLibrary.NearlyEqual_FloatFloat` (* (`ChaosVehicleMovementComponent.GetForwardSpeed` (`self.VehicleMovementComponent`)) 0.036) 0.0 10.0)))) false false)
  (if (and (== (`self.GetInputAxisValue`) 0.0) (== (`self.GetInputAxisValue`) 0.0))
    (return)
    (else
      ;[0 0.1212 1] First Person Camera
      (`SceneComponent.K2_SetRelativeRotation` _spring_arm_first_person_camera (`KismetMathLibrary.RInterpTo` (`SceneComponent.RelativeRotation` _spring_arm_first_person_camera) (`KismetMathLibrary.MakeRotator` 0.0 (`KismetMathLibrary.FClamp` (+ _relativerotation_pitch (* (`self.GetInputAxisValue`) 2.0)) -40.0 10.0) (`KismetMathLibrary.FClamp` (+ _relativerotation_yaw (* (`self.GetInputAxisValue`) 2.0)) -110.0 160.0)) (`GameplayStatics.GetWorldDeltaSeconds`) 8.0) false false)
      ;;[1 0 0.901] Look Back Camera Position
      (`SceneComponent.K2_SetRelativeLocation` _spring_arm_first_person_camera (`KismetMathLibrary.MakeVector` _relativelocation_x (`KismetMathLibrary.MapRangeClamped` _relativerotation_yaw 70.0 170.0 -25.0 -5.0) _relativelocation_z) false false)
      (return))))

(fn `Set_Start_Engine_Input`
  (if (not (`self.bIs_Engine_Start?`))
    ;[0 0.004799 1] Engine Start
    (`/Engine/EditorBlueprintResources/StandardMacros.DoOnce` false :!label _label
      (:`Completed`
        (bind _output_get (set `self.bIs_Engine_Start?` true))
        (`ActorComponent.SetActive` (`self.Audio_Start_Engine`) true false)
        (`KismetSystemLibrary.PrintString` (`KismetStringLibrary.Concat_StrStr` "ENGINE START: " (`KismetStringLibrary.Conv_BoolToString` _output_get)) true false (struct :`R` 1.0 :`G` 0.027671 :`A` 1.0))
        (goto _label :!via `Reset`)))
    (else
      ;[1 0.005134 0] Engine Off
      (bind _output_get_2 (set `self.bIs_Engine_Start?` false))
      (`KismetSystemLibrary.PrintString` (`KismetStringLibrary.Concat_StrStr` "ENGINE OFF: " (`KismetStringLibrary.Conv_BoolToString` _output_get_2)) true false (struct :`G` 0.26736 :`B` 1.0 :`A` 1.0)))))

(fn `Set_Switch_Camera`
  (params (NewParam :type Boolean))
  (bind _first_person_camera (`self.First_Person_Camera`))
  (bind _tp_camera (`self.TP_Camera`))
  ;[1 0.01308 0 1 30] If First Person Camera Activate?
  (set `self.bIs_First_Person_Camera?` (not (`self.bIs_First_Person_Camera?`)))
  (if (`self.bIs_First_Person_Camera?`)
    (`ActorComponent.SetActive` _first_person_camera true false)
    (`ActorComponent.SetActive` _tp_camera false false)
    (else
      (`ActorComponent.SetActive` _first_person_camera false false)
      (`ActorComponent.SetActive` _tp_camera true false))))

(fn `Update_Camera_Zoom`
  (locals (Temp_Current_Zoom :type "Float (single-precision)" :default 0.0))
  (bind _tp_springarm (`self.TP_SpringArm`))
  ;[0 0.25 1] Update Camera Zoom
  (set `local.Temp_Current_Zoom` (`SpringArmComponent.TargetArmLength` _tp_springarm))
  (set `SpringArmComponent.TargetArmLength` (`KismetMathLibrary.FInterpTo` (`local.Temp_Current_Zoom`) (* (`self.Camera_Zoom_Step`) (`self.Camera_Zoom_Multiplier`)) (`GameplayStatics.GetWorldDeltaSeconds`) 1.0) _tp_springarm))

(fn `UserConstructionScript`)