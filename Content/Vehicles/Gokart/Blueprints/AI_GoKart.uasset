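; AI_GoKart is an AI-driven go-kart vehicle that follows a spline path at a constant half throttle set on BeginPlay.
; Each Tick steers toward a look-ahead point, found by projecting along the nearest spline tangent and snapping back onto the ActivePath spline.
; GetPath maps the yaw difference to that point into a clamped steering input for the VehicleMovementComponent.
; The construction script tints the body through a dynamic material and can hide the driver mannequin.
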(event `self.ReceiveBeginPlay`
  (`ChaosVehicleMovementComponent.SetThrottleInput` (`self.VehicleMovementComponent`) 0.5))

(event `self.ReceiveTick`
  (params (DeltaSeconds :type "Float (single-precision)"))
  (bind _returnvalue (`self.GetPath`))
  (`ChaosVehicleMovementComponent.SetSteeringInput` (`self.VehicleMovementComponent`) _returnvalue))

(fn `GetPath`
  (returns (ReturnValue :type "Float (double-precision)"))
  (bind _returnvalue (`self.K2_GetActorLocation`))
  (bind _splinepath (`/Game/Vehicles/Gokart/Blueprints/ai_comp/path.SplinePath` (`self.ActivePath`)))
  (bind (_returnvalue_roll _returnvalue_pitch _returnvalue_yaw) (`KismetMathLibrary.BreakRotator` (`KismetMathLibrary.NormalizedDeltaRotator` (`KismetMathLibrary.FindLookAtRotation` _returnvalue (`SplineComponent.FindLocationClosestToWorldLocation` _splinepath (+ (* (`KismetMathLibrary.Normal` (`SplineComponent.FindTangentClosestToWorldLocation` _splinepath _returnvalue "World")) 200.0) _returnvalue) "World")) (`self.K2_GetActorRotation`))))
  (return (`KismetMathLibrary.MapRangeClamped` _returnvalue_yaw -90.0 90.0 -1.0 1.0)))

(fn `UserConstructionScript`
  (`|ExecutionSequence`
    (:`then_0`
      (`/Engine/EditorBlueprintResources/StandardMacros.IsValid` (`self.BodyMat`)
        (:`Is Not Valid`
          (bind _returnvalue (`PrimitiveComponent.CreateDynamicMaterialInstance` (`self.Mesh`) 0 null "None"))
          (set `self.BodyMat` _returnvalue))))
    (:`then_1`
      (`MaterialInstanceDynamic.SetVectorParameterValue` (`self.BodyMat`) "Base Color" (`self.Color`)))
    (:`then_2`
      (if (not (`self.ShowDriver`))
        (`SceneComponent.SetVisibility` (`self.Mannequin`) false false)))))