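; AI-driven Chaos wheeled car that follows a spline path at a constant throttle set on BeginPlay.
; Each tick, GetPath looks toward the spline point nearest a short tangent-based lookahead and maps the yaw difference to steering input.
; Player-car graphs for input, cameras, speedometer HUD, skidmarks and speed-based energy torque are also present, but the event graph shown never calls them.
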(event `self.ReceiveBeginPlay`
  (`ChaosVehicleMovementComponent.SetThrottleInput` (`self.VehicleMovementComponent`) 0.5))

(event `self.ReceiveTick`
  (params (DeltaSeconds :type "Float (single-precision)"))
  (bind _returnvalue (`self.Get Path`))
  (`ChaosVehicleMovementComponent.SetSteeringInput` (`self.VehicleMovementComponent`) _returnvalue))

(fn `accel1`
  (set `self.Forward?` true))

(fn `activate nos1`
  (`ActorComponent.Activate` (`self.Exhaustt`) true))

(fn `Camera_Input`
  (bind _returnvalue (`GameplayStatics.GetPlayerController` 0))
  (bind (_returnvalue_roll _returnvalue_pitch _returnvalue_yaw) (`KismetMathLibrary.BreakRotator` (`SceneComponent.K2_GetComponentRotation` (`self.RearCameraRef`))))
  (bind (_returnvalue_roll_2 _returnvalue_pitch_2 _returnvalue_yaw_2) (`KismetMathLibrary.BreakRotator` (`SceneComponent.K2_GetComponentRotation` (`self.MainCameraRef`))))
  (`SceneComponent.K2_AddRelativeRotation` (`self.MainSpringArm`) (`KismetMathLibrary.MakeRotator` 0.0 (`self.GetInputAxisValue`) (`self.GetInputAxisValue`)) false false)
  (if (> (`ChaosVehicleMovementComponent.GetForwardSpeed` (`self.VehicleMovementComponent`)) 1000.0)
    (if (not (or (`PlayerController.IsInputKeyDown` _returnvalue "Up") (`PlayerController.IsInputKeyDown` _returnvalue "Left") (`PlayerController.IsInputKeyDown` _returnvalue "Right") (`PlayerController.IsInputKeyDown` _returnvalue "Down") (`self.Customization?`)))
      (`SceneComponent.K2_SetWorldRotation` (`self.MainSpringArm`) (`KismetMathLibrary.MakeRotator` _returnvalue_roll_2 _returnvalue_pitch_2 _returnvalue_yaw_2) false false)
      (`SceneComponent.K2_SetWorldRotation` (`self.InteriorSpringArm`) (`KismetMathLibrary.MakeRotator` _returnvalue_roll_2 _returnvalue_pitch_2 _returnvalue_yaw_2) false false))
    (elif (< (`ChaosVehicleMovementComponent.GetForwardSpeed` (`self.VehicleMovementComponent`)) -500.0)
      (`SceneComponent.K2_SetWorldRotation` (`self.MainSpringArm`) (`KismetMathLibrary.MakeRotator` _returnvalue_roll _returnvalue_pitch _returnvalue_yaw) false false))))

(fn `Car_Sound`
  (`AudioComponent.SetFloatParameter` (`self.EngineSound`) "RPM" (`ChaosVehicleMovementComponent.GetForwardSpeed` (`self.VehicleMovementComponent`))))

(fn `De-Activate nos`
  (`ActorComponent.Deactivate` (`self.Exhaustt`)))

(fn `Decel`
  (set `self.Forward?` false))

(fn `Drift1`
  (params (self2 :type "ChaosVehicleMovementComponent Object Reference"))
  (`ChaosVehicleMovementComponent.SetHandbrakeInput` self2 true)
  (set `self.HandBrake?` true))

(fn `driftStop1`
  (returns (VehicleMovementComponent :type "ChaosVehicleMovementComponent Object Reference"))
  (bind _vehiclemovementcomponent (`self.VehicleMovementComponent`))
  (`ChaosVehicleMovementComponent.SetHandbrakeInput` _vehiclemovementcomponent false)
  (set `self.HandBrake?` false)
  (return _vehiclemovementcomponent))

(fn `event tick checker1`
  (params (InputPin :type "Float (single-precision)"))
  (bind _tireskidactive_ (`self.TireSkidActive?`))
  (bind _mesh (`self.Mesh`))
  (bind _tireskidleft (`self.TireSkidLeft`))
  (bind _tirefloor_ (`self.TireFloor?`))
  (bind _tireskidright (`self.TireSkidRight`))
  (bind _back_lights__group (`self.BACK LIGHTS  GROUP`))
  (bind _vehiclemovementcomponent (`self.VehicleMovementComponent`))
  (bind _returnvalue (`ChaosVehicleMovementComponent.GetForwardSpeed` (`self.VehicleMovementComponent`)))
  (bind _returnvalue_2 (`KismetMathLibrary.FClamp` (/ (`self.VehicleSpeed`) 30.0) 80.0 95.0))
  (bind _returnvalue_3 (* (`KismetMathLibrary.FClamp` (/ (- (`KismetMathLibrary.Abs` (`ChaosVehicleMovementComponent.GetForwardSpeed` (`self.VehicleMovementComponent`))) 55.0) 400.0) 0.0 0.7) (`KismetMathLibrary.Conv_BoolToDouble` (`self.HandBrake?`))))
  (`|ExecutionSequence`
    (:`then_0`
      (`self.Vehicle_Inputs`)
      (`self.Camera_Input`)
      (`self.InteriorCamera_Input`)
      (`self.SteeringWheelRotation` 0.0)
      (`self.Speedometer`)
      (`self.Gear&RPMSetup`)
      (`self.Car_Sound`)
      (if (> (`ChaosVehicleMovementComponent.GetForwardSpeed` (`self.VehicleMovementComponent`)) 2500.0)
        (bind _output_get (set `self.MainCamera` (`self.MainCamera`)))
        (bind _output_get_2 (set `self.FieldOfView` _returnvalue_2))
        (`CameraComponent.SetFieldOfView` _output_get _output_get_2)
        (else
          (bind _output_get_3 (set `self.MainCamera` (`self.MainCamera`)))
          (bind _output_get_4 (set `self.FieldOfView` _returnvalue_2))
          (`CameraComponent.SetFieldOfView` _output_get_3 _output_get_4))))
    (:`then_1`
      (`self.TireGroundCheck`)
      (if (`self.TireSkid?`)
        (bind _returnvalue_4 (`PrimitiveComponent.GetPhysicsLinearVelocity` _mesh "None"))
        (bind _y (.y (`KismetMathLibrary.LessLess_VectorRotator` _returnvalue_4 (`SceneComponent.K2_GetComponentRotation` _mesh))))
        (bind _returnvalue_5 (/ (`KismetMathLibrary.FClamp` (- (`KismetMathLibrary.Abs` (- _y 100.0)) 300.0) 0.0 1000.0) 500.0))
        (set `self.LeftValue` _returnvalue_5)
        (if _tireskidactive_
          (bind _returnvalue_6 (`KismetMathLibrary.FClamp` (+ _returnvalue_3 _returnvalue_5)))
          (`ActorComponent.SetActive` _tireskidleft (and (> _returnvalue_6 0.0) _tirefloor_) false)
          (`ActorComponent.SetActive` (`self.TIRESKIDSOUND`) (and (> _returnvalue_6 0.0) _tirefloor_) false)
          (`ActorComponent.SetActive` _tireskidright (and (> _returnvalue_6 0.0) _tirefloor_) false)
          (`FXSystemComponent.SetFloatParameter` _tireskidleft "Opacity" _returnvalue_6)
          (`FXSystemComponent.SetFloatParameter` _tireskidright "Opacity" _returnvalue_6)
          (if _tireskidactive_
            (bind _returnvalue_7 (`KismetMathLibrary.FClamp` (+ _returnvalue_3 (/ (`KismetMathLibrary.FClamp` (- (`KismetMathLibrary.Abs` (+ _y 100.0)) 300.0) 0.0 1000.0) 500.0))))
            (`ActorComponent.SetActive` _tireskidright (and _tirefloor_ (> _returnvalue_7 0.0)) false)
            (`FXSystemComponent.SetFloatParameter` _tireskidright "Opacity" _returnvalue_7)))))
    (:`then_2`)
    (:`then_3`)
    (:`then_5`
      (if (> _returnvalue 600.0)
        (if (== _returnvalue (`KismetMathLibrary.FClamp` _returnvalue 601.0 2700.0))
          (set `self.Energyy` (`KismetMathLibrary.FClamp` (+ (`self.Energyy`) (`self.EnergyIncreaseSpeed`)) 0.0 100.0))
          (`SceneComponent.SetVisibility` _back_lights__group true false)
          (if (< (`self.Energyy`) 48.0)
            (bind _aschaos_wheeled_vehicle_movement_component (cast `ChaosWheeledVehicleMovementComponent` _vehiclemovementcomponent))
            (`ChaosWheeledVehicleMovementComponent.SetMaxEngineTorque` _aschaos_wheeled_vehicle_movement_component 1000.0)
            (else
              (bind _aschaos_wheeled_vehicle_movement_component_2 (cast `ChaosWheeledVehicleMovementComponent` _vehiclemovementcomponent))
              (`ChaosWheeledVehicleMovementComponent.SetMaxEngineTorque` _aschaos_wheeled_vehicle_movement_component_2 (`self.StandartTorque`))
              (set `self.Energy` true)))
          (else
            (set `self.Energyy` (`KismetMathLibrary.FClamp` (- (`self.Energyy`) (`self.EnergyDecreaseSpeed`)) 22.0 100.0))
            (`SceneComponent.SetVisibility` _back_lights__group false false :!label _label)
            (if (> (`self.Energyy`) 70.0)
              (bind _aschaos_wheeled_vehicle_movement_component_3 (cast `ChaosWheeledVehicleMovementComponent` _vehiclemovementcomponent))
              (`ChaosWheeledVehicleMovementComponent.SetMaxEngineTorque` _aschaos_wheeled_vehicle_movement_component_3 (`self.MaxEnergyTorque`))
              (else
                (bind _aschaos_wheeled_vehicle_movement_component_4 (cast `ChaosWheeledVehicleMovementComponent` _vehiclemovementcomponent))
                (`ChaosWheeledVehicleMovementComponent.SetMaxEngineTorque` _aschaos_wheeled_vehicle_movement_component_4 (`self.StandartTorque`))
                (set `self.Energy` false)))))
        (else
          (goto _label))))))

(fn `Gear&RPMSetup`
  (bind _vehiclemovementcomponent (`self.VehicleMovementComponent`))
  (set `self.VehicleSpeed` (`ChaosVehicleMovementComponent.GetForwardSpeed` _vehiclemovementcomponent))
  (set `self.CurrentGear` (`ChaosVehicleMovementComponent.GetCurrentGear` _vehiclemovementcomponent))
  (set `self.VehicleRPM` (`KismetMathLibrary.FInterpTo` (`self.VehicleRPM`) (`KismetMathLibrary.FClamp` (`ChaosWheeledVehicleMovementComponent.GetEngineRotationSpeed` (cast `ChaosWheeledVehicleMovementComponent` _vehiclemovementcomponent :!pure true)) 0.0 8000.0) (`GameplayStatics.GetTimeSeconds`))))

(fn `Get Path`
  (returns (ReturnValue :type "Float (double-precision)"))
  (bind _returnvalue (`self.K2_GetActorLocation`))
  (bind _splinepath (`/Game/Vehicles/PX2000/BLUEPRINTS/pathing/path.SplinePath` (`self.ActivePath`)))
  (bind (_returnvalue_roll _returnvalue_pitch _returnvalue_yaw) (`KismetMathLibrary.BreakRotator` (`KismetMathLibrary.NormalizedDeltaRotator` (`KismetMathLibrary.FindLookAtRotation` _returnvalue (`SplineComponent.FindLocationClosestToWorldLocation` _splinepath (+ (* (`KismetMathLibrary.Normal` (`SplineComponent.FindTangentClosestToWorldLocation` _splinepath _returnvalue "World")) 200.0) _returnvalue) "World")) (`self.K2_GetActorRotation`))))
  ;[0.03423 0.349 0 1 40] get path for ai
  (return (`KismetMathLibrary.MapRangeClamped` _returnvalue_yaw -90.0 90.0 -1.0 1.0)))

(fn `InteriorCamera_Input`
  (`SceneComponent.K2_AddRelativeRotation` (`self.InteriorSpringArm`) (`KismetMathLibrary.MakeRotator` 0.0 (`self.GetInputAxisValue`) (`self.GetInputAxisValue`)) false false))

(fn `NewFunction`
  (returns (ReturnValue :type "Float (double-precision)"))
  (bind _returnvalue (`self.K2_GetActorLocation`))
  (bind _splinepath (`/Game/Vehicles/PX2000/BLUEPRINTS/pathing/path.SplinePath` (`self.ActivePath`)))
  (bind (_returnvalue_roll _returnvalue_pitch _returnvalue_yaw) (`KismetMathLibrary.BreakRotator` (`KismetMathLibrary.NormalizedDeltaRotator` (`KismetMathLibrary.FindLookAtRotation` _returnvalue (`SplineComponent.FindLocationClosestToWorldLocation` _splinepath (+ (* (`KismetMathLibrary.Normal` (`SplineComponent.FindTangentClosestToWorldLocation` _splinepath _returnvalue "World")) 200.0) _returnvalue) "World")) (`self.K2_GetActorRotation`))))
  (return (`KismetMathLibrary.MapRangeClamped` _returnvalue_yaw -90.0 90.0 -1.0 1.0)))

(fn `on play create hud1`
  (bind _returnvalue (`GameplayStatics.GetPlayerController` 0))
  (bind _returnvalue_2 (`|CreateWidget` "/Game/Vehicles/PX2000/SPEEDOMETERS/HUD_PX_SPEEDOMETER.HUD_PX_SPEEDOMETER_C" _returnvalue))
  (bind _output_get (set `self.CAR SPEEDOMETER` _returnvalue_2))
  (`UserWidget.AddToViewport` _output_get 0)
  (bind _returnvalue_3 (`|CreateWidget` "/Game/Vehicles/PX2000/Widget/W_HUDLOGO.W_HUDLOGO_C" _returnvalue))
  (`UserWidget.AddToViewport` _returnvalue_3 0))

(fn `pause`
  (returns (ReturnValue :type "/Game/Vehicles/PX2000/Widget/W_CONTROLS_INGAME Object Reference"))
  (bind _returnvalue (`|CreateWidget` "/Game/Vehicles/PX2000/Widget/W_CONTROLS_INGAME.W_CONTROLS_INGAME_C" (`GameplayStatics.GetPlayerController` 0)))
  (`UserWidget.AddToViewport` _returnvalue 0)
  (return _returnvalue))

(fn `ReturnCar`
  (bind (_returnvalue_x _returnvalue_y _returnvalue_z) (`KismetMathLibrary.BreakVector` (`self.K2_GetActorLocation`)))
  (bind (_returnvalue_roll _returnvalue_pitch _returnvalue_yaw) (`KismetMathLibrary.BreakRotator` (`self.K2_GetActorRotation`)))
  (`self.K2_SetActorTransform` (`KismetMathLibrary.MakeTransform` (`KismetMathLibrary.MakeVector` _returnvalue_x _returnvalue_y (+ _returnvalue_z 200.0)) (`KismetMathLibrary.MakeRotator` 0.0 0.0 _returnvalue_yaw)) false true))

(fn `Speedometer`
  (bind _vehiclerpm (`self.VehicleRPM`))
  (bind _car_speedometer (`self.CAR SPEEDOMETER`))
  (bind _returnvalue (`ChaosVehicleMovementComponent.GetForwardSpeed` (`self.VehicleMovementComponent`)))
  (bind _returnvalue_2 (`KismetMathLibrary.FFloor` (`KismetMathLibrary.Abs` (* _returnvalue 0.022))))
  (bind _returnvalue_3 (`KismetMathLibrary.FFloor` (`KismetMathLibrary.Abs` (* _returnvalue 0.036))))
  (`|ExecutionSequence`
    (:`then_0`
      (if (`self.KmhOrMhp?`)
        (set `/Game/Vehicles/PX2000/SPEEDOMETERS/HUD_PX_SPEEDOMETER.SpeedHUD` _returnvalue_3 _car_speedometer)
        (else
          (set `/Game/Vehicles/PX2000/SPEEDOMETERS/HUD_PX_SPEEDOMETER.SpeedHUD` _returnvalue_2 (`self.CAR SPEEDOMETER`))))
      (set `/Game/Vehicles/PX2000/SPEEDOMETERS/HUD_PX_SPEEDOMETER.RPM` _vehiclerpm _car_speedometer)
      (set `self.Gear` (`KismetTextLibrary.Conv_StringToText` (`self.GearDispText`)))
      (if (`self.KmhOrMhp?`)
        (bind _foundwidgets (`WidgetBlueprintLibrary.GetAllWidgetsOfClass` "/Game/Vehicles/PX2000/SPEEDOMETERS/HUD_PX_SPEEDOMETER_INT.HUD_PX_SPEEDOMETER_INT_C" false))
        (bind _output_get (set `self.CAR SPEEDOMETER INT` (`|GetArrayItem` _foundwidgets)))
        (set `/Game/Vehicles/PX2000/SPEEDOMETERS/HUD_PX_SPEEDOMETER_INT.RPM` _vehiclerpm _output_get)
        (set `/Game/Vehicles/PX2000/SPEEDOMETERS/HUD_PX_SPEEDOMETER_INT.SpeedHUD` _returnvalue_3 _output_get)
        (else
          (set `/Game/Vehicles/PX2000/SPEEDOMETERS/HUD_PX_SPEEDOMETER_INT.SpeedHUD` _returnvalue_2 _output_get)
          (set `/Game/Vehicles/PX2000/SPEEDOMETERS/HUD_PX_SPEEDOMETER_INT.RPM` _vehiclerpm _output_get))))
    (:`then_1`
      (bind _output_get_2 (set `self.CurrentGear` (`self.CurrentGear`)))
      (if (< _output_get_2 0)
        (set `self.GearDispText` "R")
        (elif (> (`self.CurrentGear`) 0)
          (set `self.GearDispText` (`KismetStringLibrary.Conv_IntToString` (`self.CurrentGear`)))
          (else
            (set `self.GearDispText` "N")))))))

(fn `SteeringWheelRotation`
  (params (DeltaSec :type "Float (double-precision)"))
  (bind _steeringwheel (`self.SteeringWheel`))
  (bind _aschaos_wheeled_vehicle_movement_component (cast `ChaosWheeledVehicleMovementComponent` (`self.VehicleMovementComponent`)))
  (`|ExecutionSequence`
    (:`then_0`
      (bind _wheels (`ChaosWheeledVehicleMovementComponent.Wheels` _aschaos_wheeled_vehicle_movement_component))
      (bind _returnvalue (`ChaosVehicleWheel.GetSteerAngle` (`|GetArrayItem` _wheels)))
      (bind _returnvalue_2 (`ChaosVehicleWheel.GetSteerAngle` (`|GetArrayItem` _wheels 1)))
      (bind _returnvalue_3 (`KismetMathLibrary.SelectFloat` _returnvalue _returnvalue_2 (>= (`KismetMathLibrary.Abs` _returnvalue) (`KismetMathLibrary.Abs` _returnvalue_2))))
      (`SceneComponent.K2_SetRelativeRotation` _steeringwheel (`KismetMathLibrary.MakeRotator` _returnvalue_3) false false))
    (:`then_1`
      (`SceneComponent.K2_SetRelativeRotation` _steeringwheel (`KismetMathLibrary.MakeRotator` _returnvalue_3) false false))))

(fn `TireGroundCheck`
  (bind _returnvalue_location (`KismetMathLibrary.BreakTransform` (`SceneComponent.K2_GetComponentToWorld` (`self.SkidmarkFloorCheck`))))
  (bind (_outhit _returnvalue) (`KismetSystemLibrary.LineTraceSingle` (+ _returnvalue_location (0.0 0.0 0.0)) (- _returnvalue_location (0.0 0.0 30.0)) "TraceTypeQuery1"))
  (set `self.TireFloor?` _returnvalue))

(fn `unpause`
  (params (self2 :type "Widget Object Reference"))
  (`Widget.RemoveFromParent` self2))

(fn `UserConstructionScript`)

(fn `Vehicle_Inputs`
  (bind _vehiclemovementcomponent (`self.VehicleMovementComponent`))
  ;[0 0 0 1 30] VEHICLE INPUTS
  (`ChaosVehicleMovementComponent.SetBrakeInput` _vehiclemovementcomponent (`self.GetInputAxisValue`))
  (`ChaosVehicleMovementComponent.SetSteeringInput` _vehiclemovementcomponent (`self.GetInputAxisValue`))
  (`ChaosVehicleMovementComponent.SetThrottleInput` _vehiclemovementcomponent (`self.GetInputAxisValue`))
  (bind _returnvalue (`ChaosVehicleMovementComponent.GetBrakeInput` (`self.VehicleMovementComponent`)))
  (set `self.Brake` _returnvalue))