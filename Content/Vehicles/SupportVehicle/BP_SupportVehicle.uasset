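; BP_SupportVehicle is a support vehicle Blueprint that lets the player cycle between three camera views.
; BeginPlay gathers its three camera components into a Cameras array.
; The ChangePerspective input advances the ActiveCamera index, deactivates every camera, then activates the one at that index.
; The wrap check compares array length with the next index inclusively, so the index can step one past the last camera before resetting to zero.
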(event `self.ReceiveBeginPlay`
  (bind _cameras (`self.Cameras`))
  (`KismetArrayLibrary.Array_Add` _cameras (`self.Camera`))
  (`KismetArrayLibrary.Array_Add` _cameras (`self.Camera_2`))
  (`KismetArrayLibrary.Array_Add` _cameras (`self.Camera_3`)))

(event `InputAction|ChangePerspective`
  (params (Key :type "Key Structure"))
  (bind _cameras (`self.Cameras`))
  (:`Pressed`
    (if (>= (`KismetArrayLibrary.Array_Length` (`self.Cameras`)) (+ (`self.ActiveCamera`) 1))
      (set `self.ActiveCamera` (+ (`self.ActiveCamera`) 1))
      (else
        (set `self.ActiveCamera` 0)))
    (for _array_element _cameras
      (`ActorComponent.SetActive` _array_element false false))
    (`ActorComponent.SetActive` (`|GetArrayItem` _cameras (`self.ActiveCamera`)) true false)))

(fn `UserConstructionScript`
  (`parent.UserConstructionScript`))