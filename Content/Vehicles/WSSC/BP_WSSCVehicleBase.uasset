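; Base vehicle Blueprint for WSSC vehicles that handles player input for switching camera views and vehicles.
; ChangePerspective increments the active index, deactivates every camera in the Cameras array and activates the indexed one, though its bounds check lets the index run one past the end before resetting.
; ChangeVehicle delegates to SwitchVehicle on BP_DefaultGameMode.
; The nodes adding three cameras to the array are disconnected, and construction only calls the parent.
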(event `InputAction|ChangePerspective`
  (params (Key :type "Key Structure"))
  (bind _cameras (`self.Cameras`))
  (:`Pressed`
    (if (>= (`KismetArrayLibrary.Array_Length` (`self.Cameras`)) (+ (`self.ActiveCamera`) 1))
      (set `self.ActiveCamera` (+ (`self.ActiveCamera`) 1))
      (else
        (set `self.ActiveCamera` 0)))
    (for _array_element _cameras
      (`ActorComponent.SetActive` _array_element false false))
    (`ActorComponent.SetActive` (`|GetArrayItem` _cameras (`self.ActiveCamera`)) true false)))

(event `InputAction|ChangeVehicle`
  (params (Key :type "Key Structure"))
  (:`Pressed`
    (bind _asbp_default_game_mode (cast `/Game/_Game/Blueprint/GameMode/BP_DefaultGameMode` (`GameplayStatics.GetGameMode`)))
    (`/Game/_Game/Blueprint/GameMode/BP_DefaultGameMode.SwitchVehicle` _asbp_default_game_mode)))

(fn `UserConstructionScript`
  (`parent.UserConstructionScript`))