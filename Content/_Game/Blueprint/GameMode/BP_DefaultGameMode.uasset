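; Default game mode that lets the first player cycle through a list of vehicles in place.
; SwitchVehicle looks up the current pawn's class in the Vehicles array, destroys that pawn and spawns the next class at its transform, wrapping around by modulo.
; It calls SpawnDefaultController on the new actor's instigator, then player controller 0 possesses the new actor if it is a WheeledVehiclePawn.
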(event `self.ReceiveBeginPlay`)

(fn `SwitchVehicle`
  (bind _returnvalue (`GameplayStatics.GetPlayerPawn` 0))
  (bind _vehicles (`self.Vehicles`))
  (`KismetSystemLibrary.PrintString` "pressed")
  (bind _result (`/Engine/EditorBlueprintResources/StandardMacros.IncrementInt` (`KismetArrayLibrary.Array_Find` _vehicles (`GameplayStatics.GetObjectClass` _returnvalue)))
    (:`  `
      (set `self.NextSpawnLocation` (`self.GetTransform` _returnvalue))
      (`self.K2_DestroyActor` _returnvalue)
      (bind _returnvalue_2 (`|SpawnActorFromClass` (`|GetArrayItem` (`self.Vehicles`) (mod _result (`KismetArrayLibrary.Array_Length` _vehicles))) (`self.NextSpawnLocation`) "AlwaysSpawn" "OverrideRootScale" null null))
      (`Pawn.SpawnDefaultController` (`Actor.Instigator` _returnvalue_2))
      (bind _aswheeled_vehicle_pawn (cast `WheeledVehiclePawn` _returnvalue_2))
      (`Controller.Possess` (`GameplayStatics.GetPlayerController` 0) _aswheeled_vehicle_pawn))))

(fn `UserConstructionScript`)